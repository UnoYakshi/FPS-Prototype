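; TargetDummy_BP is an interactive target dummy that inherits its TurnOn and TurnOff behavior from a parent class.
; Each Tick while IsHit is false, it runs a DelayTime delay and then calls TurnOff.
; The TurnOn and TurnOff overrides only forward to the parent, and the TurnOn call in the event graph is unconnected, so it never runs.
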(event EventBeginPlay)

(event Collision|EventActorBeginOverlap
  (params (OtherActor :type Actor%20Object%20Reference)))

(event EventTick
  (params (DeltaSeconds :type Float%20%28single-precision%29))
  (if (not (Variables|Default|GetbIsHit))
    (Utilities|FlowControl|Delay (Variables|Default|GetDelayTime))
    (CallFunction|TurnOff)))

(event Collision|EventActorEndOverlap
  (params (OtherActor :type Actor%20Object%20Reference)))

(fn ConstructionScript)

(fn Turnon
  (bind _returnvalue (|CallParentFunction))
  (return _returnvalue))

(fn TurnOff
  (bind _returnvalue (|CallParentFunction))
  (return _returnvalue))