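; Interactive door Blueprint that toggles between open and closed when used, with no movement or animation.
; OnUse calls its parent, then runs TurnOn or TurnOff based on IsOpen and flips that flag.
; TurnOn applies the plain orange material and disables collision on Block, while TurnOff applies the transparent orange material and restores query and physics collision.
; Both set and immediately clear IsUsed, and the event graph is inactive.
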(event EventBeginPlay
  (|CallParentFunction) ; This node is disabled and will not be called.\nDrag off pins to build functionality.
)

(event Collision|EventActorBeginOverlap
  (params (OtherActor :type Actor%20Object%20Reference))
  (|CallParentFunction OtherActor) ; This node is disabled and will not be called.\nDrag off pins to build functionality.
)

(event EventTick
  (params (DeltaSeconds :type Float%20%28single-precision%29))
  (|CallParentFunction DeltaSeconds) ; This node is disabled and will not be called.\nDrag off pins to build functionality.
)

(fn ConstructionScript
  (|CallParentFunction))

(fn OnUse
  (params (Initiator :type Actor%20Object%20Reference))
  (bind _returnvalue (|CallParentFunction Initiator))
  (if (Variables|Default|GetbIsOpen)
    (CallFunction|TurnOff)
    (else
      (CallFunction|Turnon)))
  (Variables|Default|SetbIsOpen (not (Variables|Default|GetbIsOpen)))
  (return _returnvalue))

(fn Turnon
  (Variables|Default|SetbIsUsed true)
  (Rendering|Material|SetMaterial (Variables|Default|GetStaticMesh) 0 "/Game/DesignTools/Materials/Orange_Plain_MI.Orange_Plain_MI")
  (Collision|SetCollisionEnabled (Variables|Default|GetBlock) "NoCollision")
  (bind _output_get (Variables|Default|SetbIsUsed false))
  (return _output_get))

(fn TurnOff
  (Variables|Default|SetbIsUsed true)
  (Rendering|Material|SetMaterial (Variables|Default|GetStaticMesh) 0 "/Game/DesignTools/Materials/Orange_Transparent_MI.Orange_Transparent_MI")
  (Collision|SetCollisionEnabled (Variables|Default|GetBlock) "QueryAndPhysics")
  (bind _output_get (Variables|Default|SetbIsUsed false))
  (return _output_get))