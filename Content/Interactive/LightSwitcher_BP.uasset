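; Light switch actor that toggles a set of lights on or off when used.
; OnUse checks IsOn and calls TurnOn or TurnOff, which set every light in the Lights array to the Intensity value or to zero.
; Both update IsOn and IsUsed, and OnUse returns the resulting IsUsed: true after switching on, false after switching off.
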(event EventBeginPlay
  (|CallParentFunction) ; This node is disabled and will not be called.\nDrag off pins to build functionality.
)

(event Collision|EventActorBeginOverlap
  (params (OtherActor :type Actor%20Object%20Reference))
  (|CallParentFunction OtherActor) ; This node is disabled and will not be called.\nDrag off pins to build functionality.
)

(event EventTick
  (params (DeltaSeconds :type Float%20%28single-precision%29))
  (|CallParentFunction DeltaSeconds) ; This node is disabled and will not be called.\nDrag off pins to build functionality.
)

(fn ConstructionScript
  (|CallParentFunction))

(fn Turnon
  (Variables|Default|SetbIsUsed true)
  (Variables|Default|SetbIsOn true)
  (for _array_element (Variables|Default|GetLights)
    (Rendering|Components|Light|SetIntensity (Variables|/Script/Engine.Light|GetLightComponent _array_element) (Variables|Default|GetIntensity)))
  (bind _output_get (Variables|Default|SetbIsUsed true))
  (return _output_get))

(fn TurnOff
  (Variables|Default|SetbIsUsed true)
  (Variables|Default|SetbIsOn false)
  (for _array_element (Variables|Default|GetLights)
    (Rendering|Components|Light|SetIntensity (Variables|/Script/Engine.Light|GetLightComponent _array_element) 0.0))
  (bind _output_get (Variables|Default|SetbIsUsed false))
  (return _output_get))

(fn OnUse
  (params (Initiator :type Actor%20Object%20Reference))
  (if (Variables|Default|GetbIsOn)
    (bind _returnvalue (CallFunction|TurnOff))
    (return _returnvalue)
    (else
      (bind _returnvalue_2 (CallFunction|Turnon))
      (return _returnvalue_2))))